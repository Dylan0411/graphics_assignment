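; Laser beam actor that stretches a cube mesh to end at whatever blocks its path.
; Tick, throttled by a 0.2-second Delay, fires an invisible Camera-channel line trace along the Arrow component's forward vector.
; The distance to the hit, or the full trace length on a miss, sets the Cube's X scale.
; Hits on the player character skip the rescale, so the player cannot cut the beam.
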(event EventTick
  (params (DeltaSeconds :type Float%20%28single-precision%29))
  (bind _arrow (Variables|Default|GetArrow))
  (bind _returnvalue (Transformation|GetWorldLocation _arrow))
  (Utilities|FlowControl|Delay 0.2)
  ;[1 1 1] fire invisible 'laser' first
  (bind (_outhit _returnvalue_2) (Collision|LineTraceByChannel _returnvalue (+ _returnvalue (* (Math|Vector|GetForwardVector _arrow) 5e+03)) "TraceTypeQuery2" false 0 "None"))
  ;[1 1 1] dont let the player break the laser
  (if (not (== (Game|GetPlayerCharacter 0) (.HitActor (Collision|BreakHitResult _outhit))))
    ;[1 1 1] scale laser mesh based on line trace distance
    (Transformation|SetWorldScale3D (Variables|Default|GetCube) (Math|Vector|MakeVector (/ (Math|Vector|VectorLength (- (.TraceStart (Collision|BreakHitResult _outhit)) (select _returnvalue_2 (.Location (Collision|BreakHitResult _outhit)) (.TraceEnd (Collision|BreakHitResult _outhit))))) 1e+02) 0.5 0.5))))

(fn ConstructionScript)