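; BP_ColourDoor is a door that crumbles when an actor tagged "Laser" enters its trigger box.
; The overlap check ignores the player character, then after a short delay disables the door's collision and hides it.
; It spawns BP_CrumbleDoor at the actor's transform in its place, then sets HasTriggered, which blocks later overlaps.
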(event OnComponentBeginOverlap(Box)
  (params (OverlappedComponent :type Primitive%20Component%20Object%20Reference) (OtherActor :type Actor%20Object%20Reference) (OtherComp :type Primitive%20Component%20Object%20Reference) (OtherBodyIndex :type Integer) (bFromSweep :type Boolean) (SweepResult :type Hit%20Result%20Structure%20%28by%20ref%29))
  (bind _door (Variables|Default|GetDoor))
  ;[1 1 1] Begin Overlap with Laser and not Player
  (if (not (Variables|Default|GethasTriggered))
    (if (!= OtherActor (Game|GetPlayerCharacter 0))
      (if (Actor|ActorHasTag OtherActor "Laser")
        (Utilities|FlowControl|Delay 1.0)
        (Collision|SetCollisionEnabled _door "NoCollision")
        (Rendering|SetVisibility _door false false)
        (Game|SpawnActorfromClass "/Game/ASSESSMENT_2/oldLab/BP_CrumbleDoor.BP_CrumbleDoor_C" (Transformation|GetActorTransform) "Undefined" "MultiplyWithRoot" 0 0)
        (Variables|Default|SethasTriggered true)))))

(event EventBeginPlay
  (Variables|Default|SethasTriggered false))

(fn ConstructionScript)