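; BP_LaserGoal is a puzzle target that swaps map sections when a laser hits it.
; A Laser-tagged overlap shows a popup, lights the sphere material and latches GoalAchieved.
; Laser exit clears popup and material but keeps the flag; other non-player overlaps invert this logic, so their exit also achieves the goal.
; Tick reapplies visibility and collision, hiding "map1" actors until achieved, then revealing them and hiding "map2".
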(event EventTick
  (params (DeltaSeconds :type Float%20%28single-precision%29))
  (if (Variables|Default|GetgoalAchieved)
    (for _array_element (Variables|Default|Getmap1Array)
      (Rendering|SetActorHiddenInGame _array_element false)
      (Collision|SetActorEnableCollision _array_element true))
    (for _array_element_2 (Variables|Default|Getmap2Array)
      (Rendering|SetActorHiddenInGame _array_element_2 true)
      (Collision|SetActorEnableCollision _array_element_2 false))
    (else
      (for _array_element_3 (Variables|Default|Getmap1Array)
        (Rendering|SetActorHiddenInGame _array_element_3 true)
        (Collision|SetActorEnableCollision _array_element_3 false)))))

(event Collision|EventActorBeginOverlap
  (params (OtherActor :type Actor%20Object%20Reference))
  (bind _goalachievedpopup (Variables|Default|GetgoalAchievedPopup))
  (bind _sphere1 (Variables|Default|GetSphere1))
  ;[1 1 1] Begin Overlap with Laser and Not Player
  (if (!= OtherActor (Game|GetPlayerCharacter 0))
    (if (Actor|ActorHasTag OtherActor "Laser")
      (UserInterface|Viewport|AddtoViewport _goalachievedpopup 0)
      (Rendering|Material|SetMaterial _sphere1 0 "/Game/ASSESSMENT_1/M_reflectorOn.M_reflectorOn")
      (Variables|Default|SetgoalAchieved true)
      (else
        ;[1 1 1] End overlap with Laser and Not Player
        (Widget|RemovefromParent _goalachievedpopup)
        (Rendering|Material|SetMaterial _sphere1 0 "/Game/ASSESSMENT_1/M_reflectorOff.M_reflectorOff")))))

(event Collision|EventActorEndOverlap
  (params (OtherActor :type Actor%20Object%20Reference))
  (bind _goalachievedpopup (Variables|Default|GetgoalAchievedPopup))
  (bind _sphere1 (Variables|Default|GetSphere1))
  ;[1 1 1] End overlap with Laser and Not Player
  (if (!= OtherActor (Game|GetPlayerCharacter 0))
    (if (Actor|ActorHasTag OtherActor "Laser")
      (Widget|RemovefromParent _goalachievedpopup)
      (Rendering|Material|SetMaterial _sphere1 0 "/Game/ASSESSMENT_1/M_reflectorOff.M_reflectorOff")
      (else
        ;[1 1 1] Begin Overlap with Laser and Not Player
        (UserInterface|Viewport|AddtoViewport _goalachievedpopup 0)
        (Rendering|Material|SetMaterial _sphere1 0 "/Game/ASSESSMENT_1/M_reflectorOn.M_reflectorOn")
        (Variables|Default|SetgoalAchieved true)))))

(event EventBeginPlay
  ;[1 1 1] Start
  (Variables|Default|SetgoalAchieved false)
  (bind _returnvalue (UserInterface|CreateWidget "/Game/ASSESSMENT_1/W_goalAchievedText.W_goalAchievedText_C"))
  (Variables|Default|SetgoalAchievedPopup _returnvalue)
  (Rendering|Material|SetMaterial (Variables|Default|GetSphere1) 0 "/Game/ASSESSMENT_1/M_reflectorOff.M_reflectorOff")
  (bind _outactors (Actor|GetAllActorswithTag "map1"))
  (Variables|Default|Setmap1Array _outactors)
  (bind _outactors_2 (Actor|GetAllActorswithTag "map2"))
  (Variables|Default|Setmap2Array _outactors_2)
  (for _array_element (Variables|Default|Getmap1Array)
    (Rendering|SetActorHiddenInGame _array_element true)
    (Collision|SetActorEnableCollision _array_element false)))

(fn ConstructionScript)