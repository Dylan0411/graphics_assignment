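; Drivable platform vehicle that starts hidden and shrunk, then appears and grows once it has touched BP_ProductionLine and AtDestinationREF reports arrival.
; Standing on it shows an enter prompt, and the interact input toggles driving by swapping pawn input, view target and widgets.
; While driving, Tick pins the player to a seat point, pushes the body with AddForce, and steers by directly rotating body and wheels.
; Another input cycles three cameras.
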(event OnComponentBeginOverlap(Cube)
  (params (OverlappedComponent :type Primitive%20Component%20Object%20Reference) (OtherActor :type Actor%20Object%20Reference) (OtherComp :type Primitive%20Component%20Object%20Reference) (OtherBodyIndex :type Integer) (bFromSweep :type Boolean) (SweepResult :type Hit%20Result%20Structure%20%28by%20ref%29))
  ;[0.2423 0.2423 0.2423] controls the size and visibility of the vehicle, its movement, displays the correct widgets, allow the player to get in and out, and toggle between 3 different cameras
  ;;[1 1 1] tell BP of the crate the vehicle is being transported in to explode
  (Utilities|Casting|CastToBP_ProductionLine OtherActor)
  (Variables|Default|SetactivateDroid true))

(event EventBeginPlay
  ;[0.2423 0.2423 0.2423] controls the size and visibility of the vehicle, its movement, displays the correct widgets, allow the player to get in and out, and toggle between 3 different cameras
  ;;[1 1 1] Start: set active camera, create widgets, enable player input, shrink vehicle to fit in crate and make it invisible
  (Variables|Default|SetSelectedcamera 1)
  (Components|Activation|SetActive (Variables|Default|GetCamera0) true false)
  (Components|Activation|SetActive (Variables|Default|GetCamera1) false false)
  (bind _returnvalue (UserInterface|CreateWidget "/Game/ASSESSMENT_2_OLD/WB_EnterVehicle.WB_EnterVehicle_C"))
  (Variables|Default|SetoutVehicleWIDGET _returnvalue)
  (bind _returnvalue_2 (UserInterface|CreateWidget "/Game/ASSESSMENT_2_OLD/WB_InVehicle.WB_InVehicle_C"))
  (Variables|Default|SetinVehicleWIDGET _returnvalue_2)
  (Variables|Default|SetplayerOnPlatform false)
  (Input|EnableInput (Game|GetPlayerController 0))
  (Transformation|SetWorldScale3D (Variables|Default|GetCube) "3.000000,1.500000,0.050000")
  (Variables|Default|SetisDriving false)
  (Rendering|SetVisibility (Variables|Default|GetCube) false false))

(event Collision|EventActorBeginOverlap
  (params (OtherActor :type Actor%20Object%20Reference))
  ;[0.2423 0.2423 0.2423] controls the size and visibility of the vehicle, its movement, displays the correct widgets, allow the player to get in and out, and toggle between 3 different cameras
  ;;[1 1 1] display prompt to get inside vehicle at the correct time
  (if (not (Variables|Default|GetisDriving))
    (if (== OtherActor (Game|Player|GetPlayerPawn 0))
      (Variables|Default|SetplayerOnPlatform true)
      (UserInterface|Viewport|AddtoViewport (Variables|Default|GetoutVehicleWIDGET) 0))))

(event EventTick
  (params (DeltaSeconds :type Float%20%28single-precision%29))
  (bind _cylinder5 (Variables|Default|GetCylinder5))
  (bind _cylinder4 (Variables|Default|GetCylinder4))
  (bind _cylinder2 (Variables|Default|GetCylinder2))
  (bind _cube (Variables|Default|GetCube))
  (bind _playerloc_cube3 (Variables|Default|GetplayerLoc_Cube3))
  (bind _moveforwardvalue (Variables|Default|GetmoveForwardValue))
  (bind _cube_2 (Variables|Default|GetCube))
  (bind _moveforwardvalue_2 (Variables|Default|GetmoveForwardValue))
  (bind _moverightvalue (Variables|Default|GetmoveRightValue))
  (bind _cube_3 (Variables|Default|GetCube))
  (bind _returnvalue (== _moveforwardvalue_2 -1.0))
  ;[0.2423 0.2423 0.2423] controls the size and visibility of the vehicle, its movement, displays the correct widgets, allow the player to get in and out, and toggle between 3 different cameras
  ;;[1 1 1] make the vehicle visible and expand it when it spawns, vehicle movement (spin all 3 wheels, rotate 2 wheels for steering, rotate vehicle body, add force to entire vehicle
  (if (Variables|Default|GetactivateDroid)
    (if (Variables|/Game/ASSESSMENT_2_OLD/BP_ProductionLine.BP_ProductionLine_C|GetatDestination (Variables|Default|GetatDestinationREF))
      (Rendering|SetVisibility (Variables|Default|GetCube2) true false)
      (Transformation|SetWorldScale3D _cube_2 (Math|Interpolation|VInterpTo (Transformation|GetWorldScale _cube_2) "4.500000,2.250000,0.375000" DeltaSeconds 1.0))
      (if (Variables|Default|GetisDriving)
        (Transformation|SetActorLocationAndRotation (Game|Player|GetPlayerPawn 0) (Transformation|GetWorldLocation _playerloc_cube3) (Transformation|GetWorldRotation _playerloc_cube3))
        (Physics|AddForce _cube_3 (* (Math|Vector|GetForwardVector _cube_3) (* _moveforwardvalue 1.5e+05)) "None" false)
        (if (== _moveforwardvalue 1.0)
          (Transformation|AddLocalRotation _cylinder5 "0.000000,1.000000,0.000000" false false)
          (elif (== _moveforwardvalue -1.0)
            (Transformation|AddLocalRotation _cylinder5 "0.000000,-1.000000,0.000000" false false)))
        (if (== _moverightvalue 1.0)
          (Transformation|SetRelativeRotation _cylinder2 "0.000000,-30.000000,90.000000" false false)
          (Transformation|SetRelativeRotation _cylinder4 "0.000000,30.000000,90.000000" false false)
          (if _returnvalue
            (Transformation|AddLocalRotation _cube "0.000000,-0.500000,0.000000" false false :!label _label)
            (else
              (Transformation|AddLocalRotation _cube "0.000000,0.500000,0.000000" false false :!label _label_2)))
          (elif (== _moverightvalue -1.0)
            (Transformation|SetRelativeRotation _cylinder2 "0.000000,30.000000,90.000000" false false)
            (Transformation|SetRelativeRotation _cylinder4 "0.000000,-30.000000,90.000000" false false)
            (if _returnvalue
              (goto _label_2)
              (else
                (goto _label)))
            (else
              (Transformation|SetRelativeRotation _cylinder2 "0.000000,0.000000,90.000000" false false)
              (Transformation|SetRelativeRotation _cylinder4 "0.000000,0.000000,90.000000" false false))))))))

(event Collision|EventActorEndOverlap
  (params (OtherActor :type Actor%20Object%20Reference))
  ;[0.2423 0.2423 0.2423] controls the size and visibility of the vehicle, its movement, displays the correct widgets, allow the player to get in and out, and toggle between 3 different cameras
  ;;[1 1 1] display prompt to get inside vehicle at the correct time
  (if (not (Variables|Default|GetisDriving))
    (if (== OtherActor (Game|Player|GetPlayerPawn 0))
      (Variables|Default|SetplayerOnPlatform false)
      (Widget|RemovefromParent (Variables|Default|GetoutVehicleWIDGET)))))

(event Input|ActionEvents|InputActionF_interactDrive
  (params (Key :type Key%20Structure :default "None"))
  (bind _returnvalue (Game|Player|GetPlayerPawn 0))
  (bind _returnvalue_2 (Game|GetPlayerController 0))
  (bind _invehiclewidget (Variables|Default|GetinVehicleWIDGET))
  (bind _outvehiclewidget (Variables|Default|GetoutVehicleWIDGET))
  ;[0.2423 0.2423 0.2423] controls the size and visibility of the vehicle, its movement, displays the correct widgets, allow the player to get in and out, and toggle between 3 different cameras
  ;;[1 1 1] switch between controlling the player and the vehicle + display the correct widget
  (:Pressed
    (if (Variables|Default|GetplayerOnPlatform)
      (if (Variables|Default|GetisDriving)
        (Input|EnableInput _returnvalue _returnvalue_2)
        (Game|Player|SetViewTargetwithBlend _returnvalue_2 _returnvalue 0.5 "VTBlend_Linear" 0.0 false)
        (Variables|Default|SetisDriving false)
        (Widget|RemovefromParent _invehiclewidget)
        (UserInterface|Viewport|AddtoViewport _outvehiclewidget 0)
        (else
          (Input|DisableInput _returnvalue _returnvalue_2)
          (Game|Player|SetViewTargetwithBlend _returnvalue_2 self 0.5 "VTBlend_Linear" 0.0 false)
          (Variables|Default|SetisDriving true)
          (UserInterface|Viewport|AddtoViewport _invehiclewidget 0)
          (Widget|RemovefromParent _outvehiclewidget))))))

(event Input|ActionEvents|InputActionQ_ToggleVehicleCamera
  (params (Key :type Key%20Structure :default "None"))
  (bind _camera0 (Variables|Default|GetCamera0))
  ;[0.2423 0.2423 0.2423] controls the size and visibility of the vehicle, its movement, displays the correct widgets, allow the player to get in and out, and toggle between 3 different cameras
  ;;[1 1 1] Toggle between 3 different cameras
  (:Pressed
    (if (== (Variables|Default|GetSelectedcamera) 0)
      (Components|Activation|SetActive (Variables|Default|GetCamera0) true false)
      (Components|Activation|SetActive (Variables|Default|GetCamera2) false false)
      (Variables|Default|SetSelectedcamera (+ (Variables|Default|GetSelectedcamera) 1) :!label _label)
      (if (> (Variables|Default|GetSelectedcamera) 2)
        (Variables|Default|SetSelectedcamera 0))
      (elif (== (Variables|Default|GetSelectedcamera) 1)
        (Components|Activation|SetActive (Variables|Default|GetCamera1) true false)
        (Components|Activation|SetActive _camera0 false false)
        (goto _label)
        (elif (== (Variables|Default|GetSelectedcamera) 2)
          (Components|Activation|SetActive (Variables|Default|GetCamera2) true false)
          (Components|Activation|SetActive _camera0 false false)
          (goto _label))))))

(event Input|AxisEvents|InputAxismoveVehicleForward
  (params (AxisValue :type Float%20%28single-precision%29))
  ;[0.2423 0.2423 0.2423] controls the size and visibility of the vehicle, its movement, displays the correct widgets, allow the player to get in and out, and toggle between 3 different cameras
  ;;[1 1 1] read Player Input
  (Variables|Default|SetmoveForwardValue AxisValue))

(event Input|AxisEvents|InputAxismoveVehicleRight
  (params (AxisValue :type Float%20%28single-precision%29))
  ;[0.2423 0.2423 0.2423] controls the size and visibility of the vehicle, its movement, displays the correct widgets, allow the player to get in and out, and toggle between 3 different cameras
  ;;[1 1 1] read Player Input
  (Variables|Default|SetmoveRightValue AxisValue))

(fn ConstructionScript)