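; BP_Laser is a laser emitter that stops updating once its linked LaserGoalREF reports the goal achieved.
; While active, Tick uses a 0.2-second Delay to throttle a Camera-channel trace from the Arrow, ignoring the player pawn, and stretches the Cube beam to the hit.
; Impacts spawn Niagara sparks and flashes, a reused heat distortion and fading burn decals when the point moves.
; Inactive lasers or "noLaserSparks" actors clear the heat effect.
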(event EventBeginPlay
  (Variables|Default|SetlaserActive true)
  (Variables|Default|SetspawnHeat false))

(event EventTick
  (params (DeltaSeconds :type Float%20%28single-precision%29))
  (bind _arrow (Variables|Default|GetArrow))
  (bind _lasergoalref (Variables|Default|GetlaserGoalREF))
  (bind _returnvalue (Transformation|GetWorldLocation _arrow))
  (if (Utilities|IsValid _lasergoalref)
    (if (not (Variables|/Game/ASSESSMENT_2_OLD/BP_LaserGoal.BP_LaserGoal_C|GetgoalAchieved _lasergoalref))
      (if (Variables|Default|GetlaserActive) :!label _label
        (Utilities|FlowControl|Delay 0.2)
        ;[1 1 1] fire invisible 'laser' first
        (bind (_outhit _returnvalue_2) (Collision|LineTraceByChannel _returnvalue (+ _returnvalue (* (Math|Vector|GetForwardVector _arrow) 8e+03)) "TraceTypeQuery2" false (Utilities|Array|MakeArray (Game|Player|GetPlayerPawn 0)) "None"))
        ;[1 1 1] scale laser mesh based on line trace distance
        (Transformation|SetWorldScale3D (Variables|Default|GetCube) (Math|Vector|MakeVector (/ (Math|Vector|VectorLength (- (.TraceStart (Collision|BreakHitResult _outhit)) (select _returnvalue_2 (.Location (Collision|BreakHitResult _outhit)) (.TraceEnd (Collision|BreakHitResult _outhit))))) 1e+02) 0.5 0.5))
        (if (Actor|ActorHasTag (.HitActor (Collision|BreakHitResult _outhit)) "noLaserSparks")
          (if (Utilities|IsValid (Variables|Default|Getheat)) :!label _label_2
            (Components|DestroyComponent (Variables|Default|Getheat))
            (Variables|Default|SetspawnHeat false))
          (else
            (bind _returnvalue_3 (Niagara|SpawnSystematLocation "/Game/ASSESSMENT_2_OLD/NS_LaserSparks.NS_LaserSparks" (.ImpactPoint (Collision|BreakHitResult _outhit))))
            (Niagara|SetNiagaraVariable(Vector3) _returnvalue_3 "User.hitNormal" (.ImpactNormal (Collision|BreakHitResult _outhit)))
            (Niagara|SpawnSystematLocation "/Game/ASSESSMENT_2_OLD/NS_LaserFlash.NS_LaserFlash" (.ImpactPoint (Collision|BreakHitResult _outhit)))
            (if (Variables|Default|GetspawnHeat)
              (Transformation|SetWorldLocation (Variables|Default|Getheat) (.ImpactPoint (Collision|BreakHitResult _outhit)) false false)
              (else
                (bind _returnvalue_4 (Niagara|SpawnSystematLocation "/Game/ASSESSMENT_2_OLD/NS_heatDistortion.NS_heatDistortion" (.ImpactPoint (Collision|BreakHitResult _outhit))))
                (Variables|Default|Setheat _returnvalue_4)
                (Variables|Default|SetspawnHeat true)))
            (if (> (Math|Vector|Distance(Vector) (.ImpactPoint (Collision|BreakHitResult _outhit)) (Variables|Default|GetlastBurnLocation)) 0.01)
              (Variables|Default|SetlastBurnLocation (.ImpactPoint (Collision|BreakHitResult _outhit)))
              (bind _returnvalue_5 (Rendering|Decal|SpawnDecalatLocation "/Game/ASSESSMENT_2_OLD/M_LaserBurnDecal.M_LaserBurnDecal" "5.000000,5.000000,5.000000" (Variables|Default|GetlastBurnLocation) (Math|Conversions|RotationFromXVector (.ImpactNormal (Collision|BreakHitResult _outhit))) 0.0))
              (Rendering|Components|Decal|SetFadeScreenSize _returnvalue_5 0.001)
              (Rendering|Components|Decal|SetFadeOut _returnvalue_5 0.0 3e+01 true))))
        (else
          (goto _label_2))))
    (else
      (goto _label))))

(fn ConstructionScript)