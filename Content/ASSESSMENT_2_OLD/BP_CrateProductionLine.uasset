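; BP_CrateProductionLine is a spawner actor that periodically produces BP_Crates at its own transform, passing each its LaserGoalREF.
; Tick polls BeginProductionLine on ProductionLineREF and starts crate spawning after a one-time 25-second delay.
; Once started, a SpawnCrate boolean paired with a 15-second Delay gates Tick so crates appear at a steady interval.
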(event EventBeginPlay
  (Variables|Default|SetspawnCrate true)
  (Variables|Default|SetstartSpawningCrates false))

(event EventTick
  (params (DeltaSeconds :type Float%20%28single-precision%29))
  (if (Variables|Default|GetstartSpawningCrates)
    (if (Variables|Default|GetspawnCrate) :!label _label
      (Game|SpawnActorfromClass "/Game/ASSESSMENT_2_OLD/BP_Crates.BP_Crates_C" (Transformation|GetActorTransform) "Undefined" "MultiplyWithRoot" 0 (Variables|Default|GetlaserGoalREF) 0)
      (Variables|Default|SetspawnCrate false)
      (Utilities|FlowControl|Delay 15.0)
      (Variables|Default|SetspawnCrate true))
    (elif (Variables|/Game/ASSESSMENT_2_OLD/BP_ProductionLine.BP_ProductionLine_C|GetbeginProductionLine (Variables|Default|GetproductionLineREF))
      (Utilities|FlowControl|Delay 25.0)
      (Variables|Default|SetstartSpawningCrates true)
      (goto _label))))

(fn ConstructionScript)