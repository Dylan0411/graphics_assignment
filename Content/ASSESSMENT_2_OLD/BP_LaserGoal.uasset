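; Laser puzzle goal actor that swaps the level from "map2" to "map1" tagged actors when a Laser-tagged actor hits it.
; Overlaps, ignoring the player, toggle the sphere's reflector material; a laser hit sets GoalAchieved after a delay.
; Tick keeps map1 hidden and non-colliding until then.
; It then steps through map2 with a delayed loop, applying glow materials, before revealing map1 and disabling map2.
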(event EventTick
  (params (DeltaSeconds :type Float%20%28single-precision%29))
  (if (Variables|Default|GetgoalAchieved)
    (if (Variables|Default|GettoggleMapChange)
      (bind _outactors (Actor|GetAllActorswithTag "map2"))
      (Variables|Default|Setmap2Array _outactors)
      (if (> (Variables|Default|GetarrayLen) (Variables|Default|GetcurrentArrayPos)) :!label _label
        (Utilities|FlowControl|Delay 0.001)
        (if (Utilities|IsValid (Actor|GetComponentbyClass (Utilities|Array|Get(acopy) (Variables|Default|Getmap2Array) (Variables|Default|GetcurrentArrayPos)) "/Script/Engine.StaticMeshComponent"))
          (Rendering|Material|SetMaterial (Actor|GetComponentbyClass (Utilities|Array|Get(acopy) (Variables|Default|Getmap2Array) (Variables|Default|GetcurrentArrayPos)) "/Script/Engine.StaticMeshComponent") 0 "/Game/ASSESSMENT_2_OLD/M_MapSwitchGlow.M_MapSwitchGlow"))
        (Variables|Default|SetcurrentArrayPos (+ (Variables|Default|GetcurrentArrayPos) 1))
        (goto _label)
        (else
          (for _array_element (Variables|Default|Getmap1Array)
            (Rendering|SetActorHiddenInGame _array_element false)
            (Collision|SetActorEnableCollision _array_element true))
          (for _array_element_2 (Variables|Default|Getmap2Array)
            (Rendering|SetActorHiddenInGame _array_element_2 true)
            (Collision|SetActorEnableCollision _array_element_2 false))))
      (else
        (Variables|Default|SettoggleMapChange true)))
    (else
      (for _array_element_3 (Variables|Default|Getmap1Array)
        (Rendering|SetActorHiddenInGame _array_element_3 true)
        (Collision|SetActorEnableCollision _array_element_3 false)))))

(event Collision|EventActorBeginOverlap
  (params (OtherActor :type Actor%20Object%20Reference))
  (bind _sphere1 (Variables|Default|GetSphere1))
  ;[1 1 1] Begin Overlap with Laser and Not Player
  (if (!= OtherActor (Game|GetPlayerCharacter 0))
    (if (Actor|ActorHasTag OtherActor "Laser")
      (Rendering|Material|SetMaterial _sphere1 0 "/Game/ASSESSMENT_1/M_ReflectorOn.M_ReflectorOn")
      (Utilities|FlowControl|Delay 1.0)
      (Variables|Default|SetgoalAchieved true)
      (else
        ;[1 1 1] End overlap with Laser and Not Player
        (Rendering|Material|SetMaterial _sphere1 0 "/Game/ASSESSMENT_1/M_ReflectorOff.M_ReflectorOff")))))

(event Collision|EventActorEndOverlap
  (params (OtherActor :type Actor%20Object%20Reference))
  (bind _sphere1 (Variables|Default|GetSphere1))
  ;[1 1 1] End overlap with Laser and Not Player
  (if (!= OtherActor (Game|GetPlayerCharacter 0))
    (if (Actor|ActorHasTag OtherActor "Laser")
      (Rendering|Material|SetMaterial _sphere1 0 "/Game/ASSESSMENT_1/M_ReflectorOff.M_ReflectorOff")
      (else
        ;[1 1 1] Begin Overlap with Laser and Not Player
        (Rendering|Material|SetMaterial _sphere1 0 "/Game/ASSESSMENT_1/M_ReflectorOn.M_ReflectorOn")
        (Utilities|FlowControl|Delay 1.0)
        (Variables|Default|SetgoalAchieved true)))))

(event EventBeginPlay
  ;[1 1 1] Start
  (Variables|Default|SetgoalAchieved false)
  (Rendering|Material|SetMaterial (Variables|Default|GetSphere1) 0 "/Game/ASSESSMENT_1/M_ReflectorOff.M_ReflectorOff")
  (bind _outactors (Actor|GetAllActorswithTag "map1"))
  (Variables|Default|Setmap1Array _outactors)
  (bind _outactors_2 (Actor|GetAllActorswithTag "map2"))
  (bind _output_get (Variables|Default|Setmap2Array _outactors_2))
  (Variables|Default|SetarrayLen (- (Utilities|Array|Length _output_get) 1))
  (for _array_element (Variables|Default|Getmap1Array)
    (Rendering|SetActorHiddenInGame _array_element true)
    (Collision|SetActorEnableCollision _array_element false)
    (Variables|Default|SettoggleMapChange false)
    (Variables|Default|SetcurrentArrayPos 0)))

(fn ConstructionScript)