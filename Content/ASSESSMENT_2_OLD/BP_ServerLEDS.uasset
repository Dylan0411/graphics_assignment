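; Server rack LED indicator Blueprint that shows whether the server selector is at the rack.
; On BeginPlay the green LED is visible and the red LED is hidden.
; CollisionZone overlap begin swaps to red and overlap end restores green by toggling component visibility.
; The overlap events do not check which actor enters, so any overlapping component triggers the swap.
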(event OnComponentBeginOverlap(collisionZone)
  (params (OverlappedComponent :type Primitive%20Component%20Object%20Reference) (OtherActor :type Actor%20Object%20Reference) (OtherComp :type Primitive%20Component%20Object%20Reference) (OtherBodyIndex :type Integer) (bFromSweep :type Boolean) (SweepResult :type Hit%20Result%20Structure%20%28by%20ref%29))
  ;[0.2423 0.2423 0.2423] Control the behaviour of the red and green leds on top of each server rack
  ;;[1 1 1] if server selector is here: hide the green led and display the red led
  (Rendering|SetVisibility (Variables|Default|GetGREENled) false false)
  (Rendering|SetVisibility (Variables|Default|GetREDled) true false))

(event OnComponentEndOverlap(collisionZone)
  (params (OverlappedComponent :type Primitive%20Component%20Object%20Reference) (OtherActor :type Actor%20Object%20Reference) (OtherComp :type Primitive%20Component%20Object%20Reference) (OtherBodyIndex :type Integer))
  ;[0.2423 0.2423 0.2423] Control the behaviour of the red and green leds on top of each server rack
  ;;[1 1 1] if server selector has gone: display the green led and hide the red led
  (Rendering|SetVisibility (Variables|Default|GetGREENled) true false)
  (Rendering|SetVisibility (Variables|Default|GetREDled) false false))

(event EventBeginPlay
  ;[0.2423 0.2423 0.2423] Control the behaviour of the red and green leds on top of each server rack
  ;;[1 1 1] Start: display green led and hide red led
  (Rendering|SetVisibility (Variables|Default|GetGREENled) true false)
  (Rendering|SetVisibility (Variables|Default|GetREDled) false false))

(fn ConstructionScript)