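; BP_ProductionLineReflector is a reflector actor that tracks two requirements for starting a production line: laser contact and player presence.
; Actor overlap events set LaserHit for actors tagged "Laser" and PlayerInsideActivationZone for the player pawn, with both cleared on BeginPlay.
; Laser contact also swaps the sphere's material between on and off.
; The Blueprint only records these flags and does not start the line itself.
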(event EventBeginPlay
  ;[0.2423 0.2423 0.2423] check requirements to start the production line (players presence and contact with the laser object)
  ;;[1 1 1] start: reset variables
  (Variables|Default|SetlaserHit false)
  (Variables|Default|SetplayerInsideActivationZone false))

(event Collision|EventActorEndOverlap
  (params (OtherActor :type Actor%20Object%20Reference))
  ;[0.2423 0.2423 0.2423] check requirements to start the production line (players presence and contact with the laser object)
  ;;[1 1 1] if laser has stopped overlapping: change material to OFF and mark this with a bool, if the player has left the activation range mark this with a second bool
  (if (Actor|ActorHasTag OtherActor "Laser")
    (Rendering|Material|SetMaterial (Variables|Default|GetSphere) 0 "/Game/ASSESSMENT_1/M_reflectorOff.M_ReflectorOff")
    (Variables|Default|SetlaserHit false)
    (elif (== OtherActor (Game|Player|GetPlayerPawn 0))
      (Variables|Default|SetplayerInsideActivationZone false))))

(event Collision|EventActorBeginOverlap
  (params (OtherActor :type Actor%20Object%20Reference))
  ;[0.2423 0.2423 0.2423] check requirements to start the production line (players presence and contact with the laser object)
  ;;[1 1 1] if laser has overlapped: change material to ON and mark this with a bool, if the player is inside the activation range mark this with a second bool
  (if (Actor|ActorHasTag OtherActor "Laser")
    (Rendering|Material|SetMaterial (Variables|Default|GetSphere) 0 "/Game/ASSESSMENT_1/M_reflectorOn.M_ReflectorOn")
    (Variables|Default|SetlaserHit true))
  (if (== OtherActor (Game|Player|GetPlayerPawn 0))
    (Variables|Default|SetplayerInsideActivationZone true)))

(fn ConstructionScript)