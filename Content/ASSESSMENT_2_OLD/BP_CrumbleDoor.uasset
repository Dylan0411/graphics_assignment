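; BP_CrumbleDoor is a door built on a Geometry Collection that crumbles and fades out once spawned.
; On BeginPlay it damages itself and creates a dynamic instance of M_DoorCrumble.
; A chain of timed delays then adjusts material parameters, changing a custom input, switching off the glow and darkening the colour to black in steps.
; The actor destroys itself at the end of the sequence.
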(event EventBeginPlay
  (bind _self self)
  (bind _geometrycollection (Variables|Default|GetGeometryCollection))
  (Game|Damage|ApplyDamage _self 5e+02 0 _self)
  (Rendering|Material|CreateDynamicMaterialInstance _geometrycollection 0 "/Game/ASSESSMENT_2_OLD/M_DoorCrumble.M_DoorCrumble" "None" :!class /Script/Engine.PrimitiveComponent)
  (Utilities|FlowControl|Delay 5.0)
  (Rendering|Material|SetScalarParameterValueonMaterials _geometrycollection "customNodeInput" 1e+02)
  (Utilities|FlowControl|Delay 5.0)
  (Rendering|Material|SetScalarParameterValueonMaterials _geometrycollection "glowAmount" 0.0)
  (Utilities|FlowControl|Delay 5.0)
  (Rendering|Material|SetVectorParameterValueonMaterials _geometrycollection "colourOfDoor" "0.010000,0.000000,0.000000")
  (Utilities|FlowControl|Delay 5.0)
  (Rendering|Material|SetVectorParameterValueonMaterials _geometrycollection "colourOfDoor" "0, 0, 0")
  (Utilities|FlowControl|Delay 5.0)
  (Actor|DestroyActor))

(fn ConstructionScript)