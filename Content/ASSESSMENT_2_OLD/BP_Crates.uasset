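; BP_Crates is a crate that slides itself toward the acid pool and turns into a floating crate there.
; Tick moves it at constant speed toward a hard-coded point and checks its distance to a second fixed point.
; Near that point it hides Cube1, spawns BP_FloatingCrates and destroys itself.
; If LaserGoalREF reports GoalAchieved, it instead destroys itself at a larger radius without spawning a replacement.
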(event EventTick
  (params (DeltaSeconds :type Float%20%28single-precision%29))
  (bind _returnvalue (Transformation|GetActorLocation))
  (bind _cube1 (Variables|Default|GetCube1))
  (bind _returnvalue_2 (Math|Vector|Distance(Vector) _returnvalue "-4493.896146,-896.934147,820.126341"))
  ;[0.2423 0.2423 0.2423] crate controller moves itself (crate) towards the acid pool, that then spawns the floating crates
  ;;[1 1 1] Move self (crate) from a to b, when reach b hide and spawn BP_FloatingCrate in its place.
  (Transformation|SetActorLocation (Math|Interpolation|VInterptoConstant _returnvalue "-5000.896146,-896.934147,820.126341" DeltaSeconds 165.0) false false)
  (if (Variables|/Game/ASSESSMENT_2_OLD/BP_LaserGoal.BP_LaserGoal_C|GetgoalAchieved (Variables|Default|GetlaserGoalREF))
    (if (>= 1.3e+03 _returnvalue_2)
      (Actor|DestroyActor))
    (elif (>= 3.6e+02 _returnvalue_2)
      (Rendering|SetVisibility _cube1 false false)
      (Collision|SetCollisionEnabled _cube1 "NoCollision")
      (if (not (Variables|Default|GetcubeSpawned))
        (Game|SpawnActorfromClass "/Game/ASSESSMENT_2_OLD/BP_FloatingCrates.BP_FloatingCrates_C" (Transformation|GetActorTransform) "Undefined" "MultiplyWithRoot" 0 0)
        (Variables|Default|SetcubeSpawned false)
        (Actor|DestroyActor)))))

(event EventBeginPlay
  ;[0.2423 0.2423 0.2423] crate controller moves itself (crate) towards the acid pool, that then spawns the floating crates
  ;;[1 1 1] Start: Set variables
  (Variables|Default|SetcubeSpawned false))

(fn ConstructionScript)