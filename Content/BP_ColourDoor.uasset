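; BP_ColourDoor is a door that opens while an actor tagged "Laser" overlaps its Box trigger, ignoring the player character.
; It opens and closes by toggling the Door component's visibility and collision rather than moving it.
; Laser overlap begin opens it and end closes it.
; Other non-player actors do the inverse, closing it on entry and opening it on exit, with no tracking of concurrent overlaps.
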(event OnComponentBeginOverlap(Box)
  (params (OverlappedComponent :type Primitive%20Component%20Object%20Reference) (OtherActor :type Actor%20Object%20Reference) (OtherComp :type Primitive%20Component%20Object%20Reference) (OtherBodyIndex :type Integer) (bFromSweep :type Boolean) (SweepResult :type Hit%20Result%20Structure%20%28by%20ref%29))
  (bind _door (Variables|Default|GetDoor))
  ;[1 1 1] Begin Overlap with Laser and not Player
  (if (!= OtherActor (Game|GetPlayerCharacter 0))
    (if (Actor|ActorHasTag OtherActor "Laser")
      (Collision|SetCollisionEnabled _door "NoCollision")
      (Rendering|SetVisibility _door false false)
      (else
        ;[1 1 1] End Overlap with Laser and not Player
        (Collision|SetCollisionEnabled _door "QueryAndPhysics")
        (Rendering|SetVisibility _door true false)))))

(event OnComponentEndOverlap(Box)
  (params (OverlappedComponent :type Primitive%20Component%20Object%20Reference) (OtherActor :type Actor%20Object%20Reference) (OtherComp :type Primitive%20Component%20Object%20Reference) (OtherBodyIndex :type Integer))
  (bind _door (Variables|Default|GetDoor))
  ;[1 1 1] End Overlap with Laser and not Player
  (if (!= OtherActor (Game|GetPlayerCharacter 0))
    (if (Actor|ActorHasTag OtherActor "Laser")
      (Collision|SetCollisionEnabled _door "QueryAndPhysics")
      (Rendering|SetVisibility _door true false)
      (else
        ;[1 1 1] Begin Overlap with Laser and not Player
        (Collision|SetCollisionEnabled _door "NoCollision")
        (Rendering|SetVisibility _door false false)))))

(fn ConstructionScript)