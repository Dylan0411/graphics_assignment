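; BP_LaserGoal is a laser target that signals a goal-achieved state when an actor tagged "Laser" overlaps it.
; On BeginPlay it creates the popup widget and sets the sphere's idle material.
; Overlap events share two branches that show or remove the popup and swap the material.
; Begin overlap ignores the player, but end overlap does not, so any non-laser actor leaving triggers the achieved state.
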(event Collision|EventActorBeginOverlap
  (params (OtherActor :type Actor%20Object%20Reference))
  (bind _goalachievedpopup (Variables|Default|GetgoalAchievedPopup))
  (bind _sphere1 (Variables|Default|GetSphere1))
  (if (!= OtherActor (Game|GetPlayerCharacter 0))
    (if (Actor|ActorHasTag OtherActor "Laser")
      (UserInterface|Viewport|AddtoViewport _goalachievedpopup 0)
      (Rendering|Material|SetMaterial _sphere1 0 "/Game/M_trippy.M_trippy")
      (else
        (Widget|RemovefromParent _goalachievedpopup)
        (Rendering|Material|SetMaterial _sphere1 0 "/Game/M_trippy1.M_trippy1")))))

(event Collision|EventActorEndOverlap
  (params (OtherActor :type Actor%20Object%20Reference))
  (bind _goalachievedpopup (Variables|Default|GetgoalAchievedPopup))
  (bind _sphere1 (Variables|Default|GetSphere1))
  (if (Actor|ActorHasTag OtherActor "Laser")
    (Widget|RemovefromParent _goalachievedpopup)
    (Rendering|Material|SetMaterial _sphere1 0 "/Game/M_trippy1.M_trippy1")
    (else
      (UserInterface|Viewport|AddtoViewport _goalachievedpopup 0)
      (Rendering|Material|SetMaterial _sphere1 0 "/Game/M_trippy.M_trippy"))))

(event EventBeginPlay
  (bind _returnvalue (UserInterface|CreateWidget "/Game/W_goalAchievedText.W_goalAchievedText_C"))
  (Variables|Default|SetgoalAchievedPopup _returnvalue)
  (Rendering|Material|SetMaterial (Variables|Default|GetSphere1) 0 "/Game/M_trippy1.M_trippy1"))

(fn ConstructionScript)