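; Robotic arm actor for a production line that animates, changes beacon materials and emits sparks on overlap.
; Actor or Box overlap plays the arm animation once and lights two beacon meshes, switching to a second lit material after five seconds.
; While the production line has not begun, Tick sets that second material lit or unlit from the reflector's laser-hit state.
; Box1 overlap spawns a delayed burst of Niagara laser sparks at randomized heights.
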(event OnComponentBeginOverlap(Box1)
  (params (OverlappedComponent :type Primitive%20Component%20Object%20Reference) (OtherActor :type Actor%20Object%20Reference) (OtherComp :type Primitive%20Component%20Object%20Reference) (OtherBodyIndex :type Integer) (bFromSweep :type Boolean) (SweepResult :type Hit%20Result%20Structure%20%28by%20ref%29))
  (Variables|Default|Setloop 5)
  (Utilities|FlowControl|Delay 0.2)
  (if (> (Variables|Default|Getloop) -1) :!label _label
    (bind _returnvalue (Niagara|SpawnSystematLocation "/Game/ASSESSMENT_2/NS_LaserSparks.NS_LaserSparks" (+ (Transformation|GetWorldLocation (Variables|Default|GetBox1)) (Math|Vector|MakeVector 0.0 0.0 (Math|Conversions|ToFloat(Integer) (Math|Random|RandomIntegerinRange 35 45)))) "45.000000,-90.000000,0.000000"))
    (Class|NiagaraComponent|SetAutoDestroy _returnvalue true)
    (Variables|Default|Setloop (- (Variables|Default|Getloop) 1))
    (goto _label)))

(event OnComponentBeginOverlap(Box)
  (params (OverlappedComponent :type Primitive%20Component%20Object%20Reference) (OtherActor :type Actor%20Object%20Reference) (OtherComp :type Primitive%20Component%20Object%20Reference) (OtherBodyIndex :type Integer) (bFromSweep :type Boolean) (SweepResult :type Hit%20Result%20Structure%20%28by%20ref%29))
  (bind _sphere (Variables|Default|GetSphere))
  (Components|Animation|PlayAnimation (Variables|Default|GetSkeletalMesh) "/Game/ASSESSMENT_2/AS_RoboticArm.AS_RoboticArm" false)
  (Rendering|Material|SetMaterial _sphere 0 "/Game/ASSESSMENT_2/SM_ServerBeacons_LIT_1.SM_ServerBeacons_LIT_1")
  (Utilities|FlowControl|Delay 5.0)
  (Rendering|Material|SetMaterial _sphere 0 "/Game/ASSESSMENT_2/SM_ServerBeacons_LIT_2.SM_ServerBeacons_LIT_2"))

(event EventBeginPlay)

(event Collision|EventActorBeginOverlap
  (params (OtherActor :type Actor%20Object%20Reference))
  (bind _sphere (Variables|Default|GetSphere))
  (Components|Animation|PlayAnimation (Variables|Default|GetSkeletalMesh) "/Game/ASSESSMENT_2/AS_RoboticArm.AS_RoboticArm" false)
  (Rendering|Material|SetMaterial _sphere 0 "/Game/ASSESSMENT_2/SM_ServerBeacons_LIT_1.SM_ServerBeacons_LIT_1")
  (Utilities|FlowControl|Delay 5.0)
  (Rendering|Material|SetMaterial _sphere 0 "/Game/ASSESSMENT_2/SM_ServerBeacons_LIT_2.SM_ServerBeacons_LIT_2"))

(event EventTick
  (params (DeltaSeconds :type Float%20%28single-precision%29))
  (bind _sphere (Variables|Default|GetSphere))
  (if (not (Variables|/Game/ASSESSMENT_2/BP_ProductionLine.BP_ProductionLine_C|GetbeginProductionLine (Variables|Default|GetproductionLineREF)))
    (if (Variables|/Game/ASSESSMENT_2/BP_ProductionLineReflector.BP_ProductionLineReflector_C|GetlaserHit (Variables|Default|GetproductionLineReflectorREF))
      (Rendering|Material|SetMaterial _sphere 0 "/Game/ASSESSMENT_2/SM_ServerBeacons_LIT_2.SM_ServerBeacons_LIT_2")
      (else
        (Rendering|Material|SetMaterial _sphere 0 "/Game/ASSESSMENT_2/SM_ServerBeacons_UNLIT_2.SM_ServerBeacons_UNLIT_2")))))

(fn ConstructionScript)