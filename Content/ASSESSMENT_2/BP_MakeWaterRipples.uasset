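; BP_MakeWaterRipples is an actor that moves its Cube component around a square loop, presumably to disturb water and create ripples, as its name suggests.
; Tick uses Delays to pace steps along +X, +Y, -X, then -Y, with the MoveForward flag switching between the outward and return pairs.
; Each step applies a single high-speed VInterpTo toward an offset from the current location, so the cube hops rather than glides.
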(event EventBeginPlay
  (Variables|Default|SetmoveForward true)
  (Variables|Default|SetspeedBewteenLocations 0.2))

(event Collision|EventActorBeginOverlap
  (params (OtherActor :type Actor%20Object%20Reference)))

(event EventTick
  (params (DeltaSeconds :type Float%20%28single-precision%29))
  (bind _cube (Variables|Default|GetCube))
  (bind _cube_2 (Variables|Default|GetCube))
  (bind _cube_3 (Variables|Default|GetCube))
  (bind _cube_4 (Variables|Default|GetCube))
  (bind _speedbewteenlocations (Variables|Default|GetspeedBewteenLocations))
  (bind _returnvalue (Transformation|GetWorldLocation _cube))
  (bind _returnvalue_2 (Transformation|GetWorldLocation _cube_2))
  (bind _returnvalue_3 (Transformation|GetWorldLocation _cube_3))
  (bind _returnvalue_4 (Transformation|GetWorldLocation _cube_4))
  (Utilities|FlowControl|Delay _speedbewteenlocations)
  (if (Variables|Default|GetmoveForward)
    (Transformation|SetWorldLocation _cube_3 (Math|Interpolation|VInterpTo _returnvalue_3 (+ _returnvalue_3 "100.000000,0.000000,0.000000") DeltaSeconds 1e+02) false false)
    (Utilities|FlowControl|Delay _speedbewteenlocations)
    (Transformation|SetWorldLocation _cube_2 (Math|Interpolation|VInterpTo _returnvalue_2 (+ _returnvalue_2 "0.000000,100.000000,0.000000") DeltaSeconds 1e+02) false false)
    (Variables|Default|SetmoveForward false)
    (else
      (Transformation|SetWorldLocation _cube_4 (Math|Interpolation|VInterpTo _returnvalue_4 (- _returnvalue_4 "100.000000,0.000000,0.000000") DeltaSeconds 1e+02) false false)
      (Utilities|FlowControl|Delay _speedbewteenlocations)
      (Transformation|SetWorldLocation _cube (Math|Interpolation|VInterpTo _returnvalue (- _returnvalue "0.000000,100.000000,0.000000") DeltaSeconds 1e+02) false false)
      (Variables|Default|SetmoveForward true))))

(fn ConstructionScript)