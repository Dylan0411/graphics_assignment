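; BP_Reflector is a laser reflector that emits its own laser while an actor tagged "Laser" overlaps it.
; Overlap events toggle a HideLaser flag and swap the sphere's on/off material.
; BeginPlay adds a child actor, cast to BP_Laser, whose visibility, collision and LaserActive state follow the flag every Tick.
; Tick also pins that laser to LaserOrigin's transform and the sphere to SphereLocation's position.
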(event EventBeginPlay
  ;[1 1 1] start
  (Variables|Default|SethideLaser true)
  (bind _returnvalue (AddComponent|AddChildActorComponent false))
  (Rendering|Material|SetMaterial (Variables|Default|GetSphere) 0 "/Game/ASSESSMENT_1/M_ReflectorOff.M_ReflectorOff"))

(event Collision|EventActorBeginOverlap
  (params (OtherActor :type Actor%20Object%20Reference))
  ;[1 1 1] Overlap events
  (if (Actor|ActorHasTag OtherActor "Laser")
    (Variables|Default|SethideLaser false)
    (Rendering|Material|SetMaterial (Variables|Default|GetSphere) 0 "/Game/ASSESSMENT_1/M_ReflectorOn.M_ReflectorOn")))

(event EventTick
  (params (DeltaSeconds :type Float%20%28single-precision%29))
  (bind _hidelaser (Variables|Default|GethideLaser))
  (bind _laserorigin (Variables|Default|GetlaserOrigin))
  ;[1 1 1] update
  (Transformation|SetWorldLocation (Variables|Default|GetSphere) (Transformation|GetWorldLocation (Variables|Default|GetSphereLocation)) false false)
  (Rendering|SetActorHiddenInGame (Variables|/Script/Engine.ChildActorComponent|GetChildActor (stale EventBeginPlay _returnvalue)) _hidelaser)
  (Collision|SetActorEnableCollision (Variables|/Script/Engine.ChildActorComponent|GetChildActor (stale EventBeginPlay _returnvalue)) (!= _hidelaser true))
  (Transformation|SetActorLocation (Variables|/Script/Engine.ChildActorComponent|GetChildActor (stale EventBeginPlay _returnvalue)) (Transformation|GetWorldLocation _laserorigin) false false)
  (Transformation|SetActorRotation (Variables|/Script/Engine.ChildActorComponent|GetChildActor (stale EventBeginPlay _returnvalue)) (Transformation|GetWorldRotation _laserorigin))
  (bind _asbp_laser (Utilities|Casting|CastToBP_Laser (Variables|/Script/Engine.ChildActorComponent|GetChildActor (stale EventBeginPlay _returnvalue))))
  (if _hidelaser
    (Variables|/Game/ASSESSMENT_2/BP_Laser.BP_Laser_C|SetlaserActive _asbp_laser false)
    (else
      (Variables|/Game/ASSESSMENT_2/BP_Laser.BP_Laser_C|SetlaserActive _asbp_laser true))))

(event Collision|EventActorEndOverlap
  (params (OtherActor :type Actor%20Object%20Reference))
  ;[1 1 1] Overlap events
  (if (Actor|ActorHasTag OtherActor "Laser")
    (Variables|Default|SethideLaser true)
    (Rendering|Material|SetMaterial (Variables|Default|GetSphere) 0 "/Game/ASSESSMENT_1/M_ReflectorOff.M_ReflectorOff")))

(fn ConstructionScript)