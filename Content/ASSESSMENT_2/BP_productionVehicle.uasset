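; BP_productionVehicle is a vehicle actor that glides between two hard-coded world positions and spawns an explosion actor near the end of its route.
; BeginPlay snaps it to the start and sets Triggered immediately, with a note to move that to a player toggle.
; Tick eases it along with VInterpTo.
; Within range of a checkpoint short of the target, it hides Cube, disables its collision and spawns BP_productionVehicleExplode once, guarded by BoxOpened.
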(event EventBeginPlay
  (Variables|Default|Settriggered false)
  (Transformation|SetActorLocation "-269.765869,-896.934147,835.082348" false false)
  (Variables|Default|SetatDestination false)
  (Variables|Default|SetboxOpened false)
  ;[1 1 1] trigger this with player toggle
  (Variables|Default|Settriggered true))

(event EventTick
  (params (DeltaSeconds :type Float%20%28single-precision%29))
  (bind _returnvalue (Transformation|GetActorLocation))
  (if (Variables|Default|Gettriggered)
    (Transformation|SetActorLocation (Math|Interpolation|VInterpTo _returnvalue "-5000.896146,-896.934147,820.126341" DeltaSeconds 0.1) false false)
    (if (>= 2e+02 (Math|Vector|Distance(Vector) _returnvalue "-4493.896146,-896.934147,820.126341"))
      (Variables|Default|SetatDestination true)
      (Rendering|SetVisibility (Variables|Default|GetCube) false false)
      (Collision|SetCollisionEnabled (Variables|Default|GetCube) "NoCollision")
      (if (not (Variables|Default|GetboxOpened))
        (Game|SpawnActorfromClass "/Game/ASSESSMENT_2/BP_productionVehicleExplode.BP_productionVehicleExplode_C" (Transformation|GetActorTransform) "Undefined" "MultiplyWithRoot" 0 0)
        (Variables|Default|SetboxOpened true)))))

(fn ConstructionScript)