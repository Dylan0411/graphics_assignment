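; Server LED prop that switches between a green and a red light when something enters its collision zone.
; On BeginPlay the green LED is visible and the red one is hidden.
; CollisionZone begin overlap shows red and end overlap restores green, with no filtering of the overlapping actor or count of multiple overlaps.
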(event OnComponentBeginOverlap(collisionZone)
  (params (OverlappedComponent :type Primitive%20Component%20Object%20Reference) (OtherActor :type Actor%20Object%20Reference) (OtherComp :type Primitive%20Component%20Object%20Reference) (OtherBodyIndex :type Integer) (bFromSweep :type Boolean) (SweepResult :type Hit%20Result%20Structure%20%28by%20ref%29))
  (Rendering|SetVisibility (Variables|Default|GetGREENled) false false)
  (Rendering|SetVisibility (Variables|Default|GetREDled) true false))

(event OnComponentEndOverlap(collisionZone)
  (params (OverlappedComponent :type Primitive%20Component%20Object%20Reference) (OtherActor :type Actor%20Object%20Reference) (OtherComp :type Primitive%20Component%20Object%20Reference) (OtherBodyIndex :type Integer))
  (Rendering|SetVisibility (Variables|Default|GetGREENled) true false)
  (Rendering|SetVisibility (Variables|Default|GetREDled) false false))

(event EventBeginPlay
  (Rendering|SetVisibility (Variables|Default|GetGREENled) true false)
  (Rendering|SetVisibility (Variables|Default|GetREDled) false false))

(fn ConstructionScript)