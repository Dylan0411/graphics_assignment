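; Robotic arm Blueprint for a production line, with animation, status lights and laser spark effects.
; An overlap on the actor or Box plays the arm animation and turns the sphere and cylinder lights green, then red after a delay.
; Until the production line begins, Tick sets the lights to red or unlit red based on the reflector's laser hit.
; Overlapping Box1 spawns a short-delayed burst of Niagara sparks at randomized heights.
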(event OnComponentBeginOverlap(Box1)
  (params (OverlappedComponent :type Primitive%20Component%20Object%20Reference) (OtherActor :type Actor%20Object%20Reference) (OtherComp :type Primitive%20Component%20Object%20Reference) (OtherBodyIndex :type Integer) (bFromSweep :type Boolean) (SweepResult :type Hit%20Result%20Structure%20%28by%20ref%29))
  (Variables|Default|Setloop 5)
  (Utilities|FlowControl|Delay 0.2)
  (if (> (Variables|Default|Getloop) -1) :!label _label
    (Development|PrintString "ZAPPP!!")
    (bind _returnvalue (Niagara|SpawnSystematLocation "/Game/ASSESSMENT_2/oldLab/NS_LaserSparks.NS_LaserSparks" (+ (Transformation|GetWorldLocation (Variables|Default|GetBox1)) (Math|Vector|MakeVector 0.0 0.0 (Math|Conversions|ToFloat(Integer) (Math|Random|RandomIntegerinRange 35 45)))) "45.000000,-90.000000,0.000000"))
    (Class|NiagaraComponent|SetAutoDestroy _returnvalue true)
    (Variables|Default|Setloop (- (Variables|Default|Getloop) 1))
    (goto _label)))

(event OnComponentBeginOverlap(Box)
  (params (OverlappedComponent :type Primitive%20Component%20Object%20Reference) (OtherActor :type Actor%20Object%20Reference) (OtherComp :type Primitive%20Component%20Object%20Reference) (OtherBodyIndex :type Integer) (bFromSweep :type Boolean) (SweepResult :type Hit%20Result%20Structure%20%28by%20ref%29))
  (bind _sphere (Variables|Default|GetSphere))
  (Components|Animation|PlayAnimation (Variables|Default|GetSkeletalMesh) "/Game/ASSESSMENT_2/newLab/Cylinder_1D9F1665_Skel_Sequence.Cylinder_1D9F1665_Skel_Sequence" false)
  (Rendering|Material|SetMaterial _sphere 0 "/Game/ASSESSMENT_2/newLab/serverGREEN_M.serverGREEN_M")
  (Utilities|FlowControl|Delay 5.0)
  (Rendering|Material|SetMaterial _sphere 0 "/Game/ASSESSMENT_2/newLab/serverRED_M.serverRED_M"))

(event EventBeginPlay)

(event Collision|EventActorBeginOverlap
  (params (OtherActor :type Actor%20Object%20Reference))
  (bind _sphere (Variables|Default|GetSphere))
  (Components|Animation|PlayAnimation (Variables|Default|GetSkeletalMesh) "/Game/ASSESSMENT_2/newLab/Cylinder_1D9F1665_Skel_Sequence.Cylinder_1D9F1665_Skel_Sequence" false)
  (Rendering|Material|SetMaterial _sphere 0 "/Game/ASSESSMENT_2/newLab/serverGREEN_M.serverGREEN_M")
  (Utilities|FlowControl|Delay 5.0)
  (Rendering|Material|SetMaterial _sphere 0 "/Game/ASSESSMENT_2/newLab/serverRED_M.serverRED_M"))

(event EventTick
  (params (DeltaSeconds :type Float%20%28single-precision%29))
  (bind _sphere (Variables|Default|GetSphere))
  (if (not (Variables|/Game/ASSESSMENT_2/oldLab/BP_productionLine.BP_productionLine_C|GetbeginProductionLine (Variables|Default|GetproductionLineREF)))
    (if (Variables|/Game/ASSESSMENT_2/oldLab/BP_productionLineReflector.BP_productionLineReflector_C|GetlaserHit (Variables|Default|GetproductionLineReflectorREF))
      (Rendering|Material|SetMaterial _sphere 0 "/Game/ASSESSMENT_2/newLab/serverRED_M.serverRED_M")
      (else
        (Rendering|Material|SetMaterial _sphere 0 "/Game/ASSESSMENT_2/newLab/UNLITserverRED_M.UNLITserverRED_M")))))

(fn ConstructionScript)