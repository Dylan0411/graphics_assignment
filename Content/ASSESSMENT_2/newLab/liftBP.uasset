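; Lift actor that serves as the level exit, sinking and ending the game once any actor overlaps it.
; Overlap sets a flag that makes Tick move it downward via VInterpTo toward a continually offset target, giving steady descent.
; The same overlap runs a delayed sequence: camera fade to full, level-complete widget (created at BeginPlay), then quit.
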(event EventBeginPlay
  (Variables|Default|SettriggerLift false)
  (bind _returnvalue (UserInterface|CreateWidget "/Game/ASSESSMENT_2/WB_levelComplete.WB_levelComplete_C"))
  (Variables|Default|SetlevelCompleteWIDGET _returnvalue))

(event Collision|EventActorBeginOverlap
  (params (OtherActor :type Actor%20Object%20Reference))
  (bind _returnvalue (Game|GetPlayerController 0))
  (Variables|Default|SettriggerLift true)
  (Utilities|FlowControl|Delay 5.0)
  (CameraFades|StartCameraFade :self (Variables|/Script/Engine.PlayerController|GetPlayerCameraManager _returnvalue) :ToAlpha 1.0 :Duration 5.0 :bHoldWhenFinished true)
  (Utilities|FlowControl|Delay 5.0)
  (UserInterface|Viewport|AddtoViewport (Variables|Default|GetlevelCompleteWIDGET) 0)
  (Utilities|FlowControl|Delay 5.0)
  (Game|QuitGame _returnvalue "Quit" false))

(event EventTick
  (params (DeltaSeconds :type Float%20%28single-precision%29))
  (bind _returnvalue (Transformation|GetActorLocation))
  (if (Variables|Default|GettriggerLift)
    (Transformation|SetActorLocation (Math|Interpolation|VInterpTo _returnvalue (+ _returnvalue "0.000000,0.000000,-5000.000000") DeltaSeconds 0.01) false false)))

(fn ConstructionScript)