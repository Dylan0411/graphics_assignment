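; BP_ProductionLineReflector is a reflector actor that tracks laser contact and player proximity, apparently for a production line puzzle.
; Overlap with an actor tagged "Laser" sets LaserHit and switches the Sphere between on and off materials.
; Overlap with the player pawn toggles PlayerInsideActivationZone.
; Both flags reset on BeginPlay and are only written here, with no movement or beam logic in this graph.
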(event EventBeginPlay
  ;[1 1 1] start
  (Variables|Default|SetlaserHit false)
  (Variables|Default|SetplayerInsideActivationZone false))

(event Collision|EventActorEndOverlap
  (params (OtherActor :type Actor%20Object%20Reference))
  ;[1 1 1] Overlap events
  (if (Actor|ActorHasTag OtherActor "Laser")
    (Rendering|Material|SetMaterial (Variables|Default|GetSphere) 0 "/Game/ASSESSMENT_1/M_ReflectorOff.M_ReflectorOff")
    (Variables|Default|SetlaserHit false)
    (elif (== OtherActor (Game|Player|GetPlayerPawn 0))
      (Variables|Default|SetplayerInsideActivationZone false))))

(event Collision|EventActorBeginOverlap
  (params (OtherActor :type Actor%20Object%20Reference))
  ;[1 1 1] Overlap events
  (if (Actor|ActorHasTag OtherActor "Laser")
    (Rendering|Material|SetMaterial (Variables|Default|GetSphere) 0 "/Game/ASSESSMENT_1/M_ReflectorOn.M_ReflectorOn")
    (Variables|Default|SetlaserHit true))
  (if (== (Game|Player|GetPlayerPawn 0) OtherActor)
    (Variables|Default|SetplayerInsideActivationZone true)))

(fn ConstructionScript)