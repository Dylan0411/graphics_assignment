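; BP_Crates is a crate actor that drifts toward a fixed world location and is replaced by a BP_floatingCrates actor near the end of its path.
; Tick eases it along with a slow VInterpTo and checks its distance to a second fixed point short of the target.
; Within range, it hides Cube1, disables its collision, spawns the replacement at its own transform and destroys itself.
; The CubeSpawned guard is never set true.
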(event EventTick
  (params (DeltaSeconds :type Float%20%28single-precision%29))
  (bind _returnvalue (Transformation|GetActorLocation))
  (bind _cube1 (Variables|Default|GetCube1))
  (Transformation|SetActorLocation (Math|Interpolation|VInterpTo _returnvalue "-5000.896146,-896.934147,820.126341" DeltaSeconds 0.05) false false)
  (if (>= 2e+02 (Math|Vector|Distance(Vector) _returnvalue "-4493.896146,-896.934147,820.126341"))
    (Rendering|SetVisibility _cube1 false false)
    (Collision|SetCollisionEnabled _cube1 "NoCollision")
    (if (not (Variables|Default|GetcubeSpawned))
      (Game|SpawnActorfromClass "/Game/ASSESSMENT_2/BP_floatingCrates.BP_floatingCrates_C" (Transformation|GetActorTransform) "Undefined" "MultiplyWithRoot" 0 0)
      (Variables|Default|SetcubeSpawned false)
      (Actor|DestroyActor))))

(event EventBeginPlay
  (Variables|Default|SetcubeSpawned false))

(fn ConstructionScript)