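; Actor that fires spark effects intermittently from three Niagara components.
; On BeginPlay it runs an endless loop that deactivates all three, then activates each in turn with a random delay of a few seconds after each one.
; The cycle restarts after the last delay, giving irregular timing between bursts.
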(event EventBeginPlay
  (bind _returnvalue (Math|Random|RandomFloatinRange 3.0 1e+01))
  (bind _niagara (Variables|Default|GetNiagara))
  (Components|Activation|Deactivate _niagara :!label _label)
  (Components|Activation|Activate _niagara false)
  (Utilities|FlowControl|Delay _returnvalue)
  (Components|Activation|Activate (Variables|Default|GetNiagara1) false)
  (Utilities|FlowControl|Delay _returnvalue)
  (Components|Activation|Activate (Variables|Default|GetNiagara2) false)
  (Utilities|FlowControl|Delay _returnvalue)
  (goto _label))

(event Collision|EventActorBeginOverlap
  (params (OtherActor :type Actor%20Object%20Reference)))

(fn ConstructionScript)