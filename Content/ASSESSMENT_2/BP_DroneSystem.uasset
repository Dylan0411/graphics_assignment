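; Drone actor that flies a droid between randomly chosen server locations (actors tagged "serverLocations") and a landing pad.
; Tick steers it by state: until the referenced laser goal is achieved it darts quickly toward the selector, afterwards it eases slowly between server and pad.
; Droid overlaps drive the rest: sparks and a re-randomized target in the initial state, later timed pauses before switching destination.
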(event OnComponentBeginOverlap(Droid)
  (params (OverlappedComponent :type Primitive%20Component%20Object%20Reference) (OtherActor :type Actor%20Object%20Reference) (OtherComp :type Primitive%20Component%20Object%20Reference) (OtherBodyIndex :type Integer) (bFromSweep :type Boolean) (SweepResult :type Hit%20Result%20Structure%20%28by%20ref%29))
  (bind _serverlocarray (Variables|Default|GetserverLocArray))
  (bind _serverlocarray_2 (Variables|Default|GetserverLocArray))
  (if (!= (Variables|Default|GetdroidState) 0)
    (if (== OtherComp (Variables|Default|GetserverSelector))
      (if (not (Variables|Default|GetserverFoundByDroid))
        (Variables|Default|SetserverFoundByDroid true)
        (Variables|Default|SetserverSelected false)
        (Variables|Default|SetdroidState 3)
        (if (not (Variables|Default|GetserverSelected))
          (Transformation|SetWorldLocation (Variables|Default|GetserverSelector) (Transformation|GetActorLocation (Utilities|Array|Get(acopy) _serverlocarray_2 (Math|Random|RandomInteger (Utilities|Array|Length _serverlocarray_2)))) false false)
          (Utilities|FlowControl|Delay 2.5)
          (Variables|Default|SetdroidState 2)))
      (elif (== OtherComp (Variables|Default|GetlandingPad))
        (Variables|Default|SetserverFoundByDroid false)
        (Utilities|FlowControl|Delay 2.5)
        (Variables|Default|SetdroidState 1)
        (Variables|Default|SetserverSelected true)
        (Variables|Default|SetserverFoundByDroid false)))
    (else
      (Niagara|SpawnSystematLocation "/Game/ASSESSMENT_2/NS_LaserSparks.NS_LaserSparks" (Transformation|GetWorldLocation (Variables|Default|GetDroid)))
      (Variables|Default|SetserverSelected false)
      (if (not (Variables|Default|GetserverSelected))
        (Transformation|SetWorldLocation (Variables|Default|GetserverSelector) (Transformation|GetActorLocation (Utilities|Array|Get(acopy) _serverlocarray (Math|Random|RandomInteger (Utilities|Array|Length _serverlocarray)))) false false)
        (Variables|Default|SetserverSelected true)))))

(event EventBeginPlay
  (bind _outactors (Actor|GetAllActorswithTag "serverLocations"))
  (Variables|Default|SetserverLocArray _outactors)
  (Transformation|SetWorldLocation (Variables|Default|GetserverSelector) (Transformation|GetActorLocation (Utilities|Array|Get(acopy) (Variables|Default|GetserverLocArray) (Math|Random|RandomInteger (Utilities|Array|Length (Variables|Default|GetserverLocArray))))) false false)
  (Variables|Default|SetserverSelected true)
  (Variables|Default|SetserverFoundByDroid false)
  (Variables|Default|SetdroidState 0))

(event Collision|EventActorBeginOverlap
  (params (OtherActor :type Actor%20Object%20Reference)))

(event EventTick
  (params (DeltaSeconds :type Float%20%28single-precision%29))
  (bind _serverselector (Variables|Default|GetserverSelector))
  (bind _landingpad (Variables|Default|GetlandingPad))
  (bind _droid (Variables|Default|GetDroid))
  (bind _droid_2 (Variables|Default|GetDroid))
  (bind _serverselector_2 (Variables|Default|GetserverSelector))
  (bind _droid_3 (Variables|Default|GetDroid))
  (bind _droid_4 (Variables|Default|GetDroid))
  (bind _droid_5 (Variables|Default|GetDroid))
  (bind _droid_6 (Variables|Default|GetDroid))
  (bind _returnvalue (Transformation|GetWorldLocation _serverselector))
  (bind _returnvalue_2 (Transformation|GetWorldLocation _droid_3))
  (bind _returnvalue_3 (Transformation|GetWorldLocation _droid))
  (bind _returnvalue_4 (Transformation|GetWorldLocation _landingpad))
  (bind _returnvalue_5 (Transformation|GetWorldLocation _serverselector_2))
  (bind _returnvalue_6 (Transformation|GetWorldLocation _droid_4))
  (if (== (Variables|Default|GetdroidState) 0)
    (if (Variables|/Game/ASSESSMENT_2/BP_LaserGoal.BP_LaserGoal_C|GetgoalAchieved (Variables|Default|GetlaserGoalREF))
      (Variables|Default|SetdroidState 1)
      (else
        (Transformation|SetWorldRotation _droid_5 (Math|Interpolation|RInterpTo (Transformation|GetWorldRotation _droid_4) (Math|Rotator|FindLookatRotation _returnvalue_6 _returnvalue_5) DeltaSeconds 5.0) false false)
        (Transformation|SetWorldLocation _droid_5 (Math|Interpolation|VInterptoConstant _returnvalue_6 _returnvalue_5 DeltaSeconds 1e+03) false false)))
    (elif (== (Variables|Default|GetdroidState) 1)
      (Transformation|SetWorldRotation _droid_6 (Math|Interpolation|RInterpTo (Transformation|GetWorldRotation _droid_3) (Math|Rotator|FindLookatRotation _returnvalue_2 _returnvalue) DeltaSeconds 5.0) false false)
      (Transformation|SetWorldLocation _droid_6 (Math|Interpolation|VInterpTo _returnvalue_2 _returnvalue DeltaSeconds 0.5) false false)
      (elif (== (Variables|Default|GetdroidState) 2)
        (Transformation|SetWorldRotation _droid_2 (Math|Interpolation|RInterpTo (Transformation|GetWorldRotation _droid) (Math|Rotator|FindLookatRotation _returnvalue_3 _returnvalue_4) DeltaSeconds 5.0) false false)
        (Transformation|SetWorldLocation _droid_2 (Math|Interpolation|VInterpTo _returnvalue_3 _returnvalue_4 DeltaSeconds 0.5) false false)
        (elif (== (Variables|Default|GetdroidState) 3)
          _)))))

(fn ConstructionScript)