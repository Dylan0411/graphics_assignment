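; BP_boxProductionLine is a crate spawner that emits BP_Crates at its own transform once the referenced production line begins.
; Tick polls the production line's BeginProductionLine flag, then after a long delay latches spawning on.
; A SpawnCrate gate with a second delay spaces out repeated spawns, printing a debug message each time.
; Each spawned crate receives the spawner's LaserGoal reference.
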(event EventBeginPlay
  (Variables|Default|SetspawnCrate true)
  (Variables|Default|SetstartSpawningCrates false))

(event EventTick
  (params (DeltaSeconds :type Float%20%28single-precision%29))
  (if (Variables|Default|GetstartSpawningCrates)
    (if (Variables|Default|GetspawnCrate) :!label _label
      (Development|PrintString "crate spawned")
      (Game|SpawnActorfromClass "/Game/ASSESSMENT_2/oldLab/BP_Crates.BP_Crates_C" (Transformation|GetActorTransform) "Undefined" "MultiplyWithRoot" 0 (Variables|Default|GetlaserGoalREF) 0)
      (Variables|Default|SetspawnCrate false)
      (Utilities|FlowControl|Delay 15.0)
      (Variables|Default|SetspawnCrate true))
    (else
      ;[1 1 1] if big crate "atdestination" bool is true
      (if (Variables|/Game/ASSESSMENT_2/oldLab/BP_productionLine.BP_productionLine_C|GetbeginProductionLine (Variables|Default|GetproductionLineREF))
        (Utilities|FlowControl|Delay 25.0)
        (Variables|Default|SetstartSpawningCrates true)
        (goto _label)))))

(fn ConstructionScript)