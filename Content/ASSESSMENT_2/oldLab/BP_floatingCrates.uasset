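; Floating crate actor that splashes down in a pool, then drifts, spins and bobs.
; The first hit on Cube latches; if it is tagged bottomOfPool, a Niagara splash spawns and floating starts after a short delay.
; Tick picks random drift and yaw speeds once, then while floating moves Cube and bobs Cube1 between top and bottom marker components using constant-speed interpolation.
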(event OnComponentHit(Cube)
  (params (HitComponent :type Primitive%20Component%20Object%20Reference) (OtherActor :type Actor%20Object%20Reference) (OtherComp :type Primitive%20Component%20Object%20Reference) (NormalImpulse :type Vector :default "0, 0, 0") (Hit :type Hit%20Result%20Structure%20%28by%20ref%29))
  (if (not (Variables|Default|GetsplashDown))
    (Variables|Default|SetsplashDown true)
    (if (Actor|ActorHasTag OtherActor "bottomOfPool")
      (bind _returnvalue (Niagara|SpawnSystematLocation "/Game/ASSESSMENT_2/oldLab/NS_Splash.NS_Splash" (Transformation|GetWorldLocation (Variables|Default|GetCube)) "90.000000,0.000000,0.000000"))
      (Class|NiagaraComponent|SetAutoDestroy _returnvalue true)
      (Utilities|FlowControl|Delay 0.5)
      (Variables|Default|SetinWater true))))

(event EventTick
  (params (DeltaSeconds :type Float%20%28single-precision%29))
  (bind _returnvalue (Math|Random|RandomFloatinRange -0.25 0.25))
  (bind _cube (Variables|Default|GetCube))
  (bind _cube1 (Variables|Default|GetCube1))
  (bind _returnvalue_2 (Transformation|GetWorldLocation _cube1))
  (if (Variables|Default|Getdrift)
    (Variables|Default|SetNSdriftSpeed _returnvalue)
    (Variables|Default|SetEWdriftSpeed _returnvalue)
    (Variables|Default|SetrotationSpeed (Math|Random|RandomFloatinRange -0.1 0.1))
    (Variables|Default|SettargetLoc (+ (Transformation|GetWorldLocation (Variables|Default|GetCube)) (Math|Vector|MakeVector (Math|Conversions|ToFloat(Integer) (Math|Random|RandomInteger 3000)) (Math|Conversions|ToFloat(Integer) (Math|Random|RandomInteger 3000)) 0.0)))
    (Variables|Default|Setdrift false))
  (if (Variables|Default|GetinWater)
    (Transformation|AddWorldOffset _cube (Math|Vector|MakeVector (Variables|Default|GetNSdriftSpeed) (Variables|Default|GetEWdriftSpeed) 0.0) false false)
    (Transformation|AddWorldRotation _cube (Math|Rotator|MakeRotator 0.0 0.0 (Variables|Default|GetrotationSpeed)) false false)
    (Transformation|SetWorldLocation (Variables|Default|GetCube1) (Math|Interpolation|VInterptoConstant _returnvalue_2 (Variables|Default|GettargetLoc) DeltaSeconds (Variables|Default|GetmovementSpeed)) false false)
    (if (Variables|Default|GetmoveUp)
      (Variables|Default|SettargetLoc (Transformation|GetWorldLocation (Variables|Default|GetCubeTopPos)))
      (if (<= (Math|Vector|Distance(Vector) _returnvalue_2 (Variables|Default|GettargetLoc)) 1.0)
        (Variables|Default|SetmoveUp false))
      (else
        (Variables|Default|SettargetLoc (Transformation|GetWorldLocation (Variables|Default|GetCubeBottomPos)))
        (if (<= (Math|Vector|Distance(Vector) _returnvalue_2 (Variables|Default|GettargetLoc)) 1.0)
          (Variables|Default|SetmoveUp true))))))

(event EventBeginPlay
  (Variables|Default|SetmoveUp true)
  (Variables|Default|SetmovementSpeed 7.0)
  (Variables|Default|SetinWater false)
  (Variables|Default|Setdrift true))

(fn ConstructionScript)