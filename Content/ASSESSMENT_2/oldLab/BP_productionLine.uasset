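; BP_productionLine is an actor that travels along a production line and breaks open near the end.
; While the player is in the referenced line's activation zone and its laser hit is set, a prompt widget shows and the interact key starts movement.
; Tick eases the actor toward a hardcoded endpoint with VInterpTo; within range it hides its cube, spawns a BP_CrumbleCrate once and flags arrival after a short delay.
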(event EventBeginPlay
  (Transformation|SetActorLocation "-269.765869,-896.934147,835.082348" false false)
  (Variables|Default|SetatDestination false)
  (Variables|Default|SetboxOpened false)
  (Variables|Default|SetbeginProductionLine false)
  (Input|EnableInput (Game|GetPlayerController 0))
  (bind _returnvalue (UserInterface|CreateWidget "/Game/ASSESSMENT_2/WB_ActivateProductionLine.WB_ActivateProductionLine_C"))
  (Variables|Default|SetactivateProductionLineWIDGET _returnvalue))

(event EventTick
  (params (DeltaSeconds :type Float%20%28single-precision%29))
  (bind _returnvalue (Transformation|GetActorLocation))
  (bind _activateproductionlinewidget (Variables|Default|GetactivateProductionLineWIDGET))
  (if (Variables|Default|GetbeginProductionLine)
    (Transformation|SetActorLocation (Math|Interpolation|VInterpTo _returnvalue "-5000.896146,-896.934147,820.126341" DeltaSeconds 0.05) false false)
    (if (>= 2e+02 (Math|Vector|Distance(Vector) _returnvalue "-4493.896146,-896.934147,820.126341"))
      (Rendering|SetVisibility (Variables|Default|GetCube) false false)
      (Collision|SetCollisionEnabled (Variables|Default|GetCube) "NoCollision")
      (if (not (Variables|Default|GetboxOpened))
        (Game|SpawnActorfromClass "/Game/ASSESSMENT_2/oldLab/BP_CrumbleCrate.BP_CrumbleCrate_C" (Transformation|GetActorTransform) "Undefined" "MultiplyWithRoot" 0 0)
        (Variables|Default|SetboxOpened true)
        (Utilities|FlowControl|Delay 0.25)
        (Variables|Default|SetatDestination true)))
    (elif (Variables|/Game/ASSESSMENT_2/oldLab/BP_productionLineReflector.BP_productionLineReflector_C|GetplayerInsideActivationZone (Variables|Default|GetProductionLineREF))
      (if (Variables|/Game/ASSESSMENT_2/oldLab/BP_productionLineReflector.BP_productionLineReflector_C|GetlaserHit (Variables|Default|GetProductionLineREF))
        (Development|PrintString "3")
        (Variables|Default|SetrequirementsMet true)
        (UserInterface|Viewport|AddtoViewport _activateproductionlinewidget 0)
        (else
          (Development|PrintString "2")
          (Variables|Default|SetrequirementsMet false)
          (Widget|RemovefromParent _activateproductionlinewidget)))
      (else
        (Development|PrintString "1")
        (Variables|Default|SetrequirementsMet false)
        (Widget|RemovefromParent _activateproductionlinewidget)))))

(event Input|ActionEvents|InputActionE_interactProductionLine
  (params (Key :type Key%20Structure :default "None"))
  (:Pressed
    (if (not (Variables|Default|GetbeginProductionLine))
      (if (Variables|Default|GetrequirementsMet)
        (Variables|Default|SetbeginProductionLine true)
        (Development|PrintString "1")
        (Variables|Default|SetrequirementsMet false)
        (Widget|RemovefromParent (Variables|Default|GetactivateProductionLineWIDGET))
        (else
          (Variables|Default|SetbeginProductionLine false))))))

(fn ConstructionScript)